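; Behavior tree service that reports to the Blackboard whether the AI-controlled Dummy is under attack.
; On search start it casts the controlled pawn to Dummy and caches the reference.
; Each tick, while that reference is valid, it copies EstaSiendoAtacado into the LoAtacan bool key.
; A SetCloseRangeBehavior helper writes an enum to BehaviorKey, though nothing in this service's event graph calls it.
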(event `self.ReceiveSearchStartAI`
  (params (OwnerController :type "AIController Object Reference") (ControlledPawn :type "Pawn Object Reference"))
  (bind _asdummy (cast `/Game/FSG/BLUEPRINTS/AI/Dummy` ControlledPawn))
  (set `self.DummyRef` _asdummy))

(event `self.ReceiveTick`
  (params (OwnerActor :type "Actor Object Reference") (DeltaSeconds :type "Float (single-precision)"))
  (bind _dummyref (`self.DummyRef`)
    (:`then`
      (`BTFunctionLibrary.SetBlackboardValueAsBool` (`self.LoAtacan?`) (`/Game/FSG/BLUEPRINTS/AI/Dummy.EstaSiendoAtacado` _dummyref)))
    (:`else`)))