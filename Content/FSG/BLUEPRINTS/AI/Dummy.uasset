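; Fighting-game dummy opponent that faces OtherActor by flipping its mesh's Y scale, takes damage and plays attacks.
; TomarDaño, unless blocking, subtracts health, plays an indexed reaction montage and triggers a delayed death sound at zero health.
; TipoAtaqueDummy maps each attack type to a montage and a ReactionInt for the player's reaction.
; Named timers clear the hit, block and crouch states; the hitbox events are empty, their spawn and destroy logic disconnected.
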(event `self.ReceiveTick`
  (params (DeltaSeconds :type "Float (single-precision)"))
  (bind (_returnvalue_x _returnvalue_y) (`KismetMathLibrary.BreakVector` (`self.K2_GetActorLocation`)))
  (bind (_returnvalue_x_2 _returnvalue_y_2) (`KismetMathLibrary.BreakVector` (`self.K2_GetActorLocation` (`self.OtherActor`))))
  (bind (_relativescale3d_x _relativescale3d_y _relativescale3d_z) (`KismetMathLibrary.BreakVector` (`SceneComponent.RelativeScale3D` (`self.Mesh`))))
  (bind (_relativescale3d_x_2 _relativescale3d_y_2 _relativescale3d_z_2) (`KismetMathLibrary.BreakVector` (`SceneComponent.RelativeScale3D` (`self.Mesh`))))
  ;[1 1 1] Para que mire hacie adelante
  (`/Engine/EditorBlueprintResources/StandardMacros.IsValid` (`self.OtherActor`)
    (:`Is Valid`
      (if (>= _returnvalue_y_2 _returnvalue_y)
        (if (`self.EstaGirado`)
          (`SceneComponent.SetRelativeScale3D` (`self.Mesh`) (`KismetMathLibrary.MakeVector` _relativescale3d_x_2 (`KismetMathLibrary.Abs` _relativescale3d_y_2) _relativescale3d_z_2))
          (set `self.EstaGirado` false))
        (elif (not (`self.EstaGirado`))
          (`SceneComponent.SetRelativeScale3D` (`self.Mesh`) (`KismetMathLibrary.MakeVector` _relativescale3d_x (* _relativescale3d_y -1.0) _relativescale3d_z))
          (set `self.EstaGirado` true))))))

(event `Validacion`
  (`KismetSystemLibrary.PrintString` "reset")
  (`self.NoEstaBloqueando`)
  (`self.NoEstaAgachado`))

(event `MUERTE`
  (`KismetSystemLibrary.Delay` 0.5)
  (`GameplayStatics.PlaySound2D` "/Game/FSG/AUDIO/SFXFALLING1.SFXFALLING1" 1.5 1.0 0.0 null null))

(event `CrearHitbox`)

(event `DestroyHitbox`
  ;[1 1 1] Destruye el hitbox (en el caso del dummy lo hace el AnimNotifyReset)
)

(fn `EstaAgachado`
  (returns (Tiempo :type "Float (double-precision)"))
  (set `self.Agacharse` true)
  (`KismetSystemLibrary.K2_ClearTimer` null "NoEstaAgachado")
  (`KismetSystemLibrary.K2_SetTimer` null "NoEstaAgachado" 1.0)
  (return (`self.Tiempo`)))

(fn `EstaBloqueando`
  (returns (Tiempo :type "Float (double-precision)"))
  (set `self.Bloqueando` true)
  (`KismetSystemLibrary.K2_ClearTimer` null "NoEstaBloqueando")
  (`KismetSystemLibrary.K2_SetTimer` null "NoEstaBloqueando" 1.0)
  (return (`self.Tiempo`)))

(fn `NoEstaAgachado`
  (set `self.Agacharse` false))

(fn `NoEstaBajoAtaque`
  (set `self.BajoAtaque` false))

(fn `NoEstaBloqueando`
  (set `self.Bloqueando` false))

(fn `TipoAtaqueDummy`
  (params (TipoAtaque :type "/Game/FSG/BLUEPRINTS/AI/Enum_DummyAtaques Enum" :default "NewEnumerator0"))
  (returns (`Duración` :type "Float (double-precision)"))
  (locals (NewDummyAtaque :type "AnimMontage Object Reference"))
  ;[1 1 1] Determina los tipos de ataques con sus respectivas reacciones por parte del player
  (set `self.Bloqueando` false)
  (switch `/Game/FSG/BLUEPRINTS/AI/Enum_DummyAtaques` TipoAtaque
    (:`NewEnumerator0`
      (set `local.NewDummyAtaque` (`|GetArrayItem` (`self.AttackMontages`)))
      (set `self.ReactionInt` 0))
    (:`NewEnumerator1`
      (set `local.NewDummyAtaque` (`|GetArrayItem` (`self.AttackMontages`) 1))
      (set `self.ReactionInt` 2))
    (:`NewEnumerator2`
      (set `local.NewDummyAtaque` (`|GetArrayItem` (`self.AttackMontages`) 2))
      (set `self.ReactionInt` 0))
    (:`NewEnumerator3`
      (set `local.NewDummyAtaque` (`|GetArrayItem` (`self.AttackMontages`) 3))
      (set `self.ReactionInt` 1))
    (:`NewEnumerator4`
      (set `local.NewDummyAtaque` (`|GetArrayItem` (`self.AttackMontages`) 4))
      (set `self.ReactionInt` 2))
    (:`NewEnumerator5`
      (set `local.NewDummyAtaque` (`|GetArrayItem` (`self.AttackMontages`) 5))
      (set `self.ReactionInt` 0))
    (:`NewEnumerator6`
      (set `local.NewDummyAtaque` (`|GetArrayItem` (`self.AttackMontages`) 6))
      (set `self.ReactionInt` 0))
    (:`NewEnumerator7`
      (set `local.NewDummyAtaque` (`|GetArrayItem` (`self.AttackMontages`) 7))
      (set `self.ReactionInt` 0))
    (:`NewEnumerator8`
      (set `local.NewDummyAtaque` (`|GetArrayItem` (`self.AttackMontages`) 8))
      (set `self.ReactionInt` 0)))
  (bind _returnvalue (`self.PlayAnimMontage` (`local.NewDummyAtaque`)))
  (return _returnvalue))

(fn `Tomar Daño`
  (params (ReactionIndex :type Integer) (`Daño` :type Integer))
  (if (not (`self.Bloqueando`))
    (set `self.BajoAtaque` true)
    (set `self.Bloqueando` false)
    (set `self.DummyHealth` (- (`self.DummyHealth`) `Daño`))
    (`KismetSystemLibrary.K2_ClearTimer` null "NoEstaBajoAtaque")
    (`self.StopAnimMontage` null)
    (bind _returnvalue (`self.PlayAnimMontage` (`|GetArrayItem` (`self.ReactionMontages`) ReactionIndex)))
    (`KismetSystemLibrary.K2_SetTimer` null "NoEstaBajoAtaque" (- _returnvalue 1.0))
    (if (<= (`self.DummyHealth`) 0)
      (set `self.Muerto` true)
      (`self.MUERTE`))))

(fn `UserConstructionScript`)