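; Melee hitbox actor for a fighting game, dealing damage between the player (FightGIrlBP) and the Dummy enemy.
; Separate player and enemy spawn events set the display material by hitbox type, then move and show the mesh at HitboxLocation.
; Each then checks overlapping actors except the owner, casts to the opposing class and calls its take-damage function with reaction index and damage.
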(event `SpawnHitbox`
  ;[1 1 1] Eventos para el jugador
  (switch `/Game/FSG/BLUEPRINTS/Enumerations/Enum_HitboxType` (`self.HitboxType`)
    (:`NewEnumerator0`
      (`PrimitiveComponent.SetMaterial` (`self.HitboxDisplay`) 0 null))
    (:`NewEnumerator1`
      (`PrimitiveComponent.SetMaterial` (`self.HitboxDisplay`) 0 null)))
  (`SceneComponent.K2_SetWorldLocation` (`self.HitboxDisplay`) (`self.HitboxLocation`) false false)
  (`SceneComponent.SetVisibility` (`self.HitboxDisplay`) true false)
  (`self.CheckCollision`))

(event `DummySpawnHitbox`
  ;[1 1 1] Eventos para el enemigo
  (switch `/Game/FSG/BLUEPRINTS/Enumerations/Enum_HitboxType` (`self.HitboxType`)
    (:`NewEnumerator0`
      (`PrimitiveComponent.SetMaterial` (`self.HitboxDisplay`) 0 null))
    (:`NewEnumerator1`
      (`PrimitiveComponent.SetMaterial` (`self.HitboxDisplay`) 0 null)))
  (`SceneComponent.K2_SetWorldLocation` (`self.HitboxDisplay`) (`self.HitboxLocation`) false false)
  (`SceneComponent.SetVisibility` (`self.HitboxDisplay`) true false)
  (`self.DummyCheckCollision`))

(event `CheckCollision`
  ;[1 1 1] Eventos para el jugador
  (for _array_element (`self.GetOverlappingActors` null)
    (if (!= _array_element (`self.GetOwner`))
      (bind _asdummy (cast `/Game/FSG/BLUEPRINTS/AI/Dummy` _array_element))
      (`/Game/FSG/BLUEPRINTS/AI/Dummy.Tomar Daño` _asdummy (`self.ReactionIndex`) (`self.HitboxDamage`)))))

(event `DummyCheckCollision`
  ;[1 1 1] Eventos para el enemigo
  (for _array_element (`self.GetOverlappingActors` null)
    (if (!= _array_element (`self.GetOwner`))
      (bind _asfight_girl_bp (cast `/Game/FSG/BLUEPRINTS/FightGIrlBP` _array_element))
      (`KismetSystemLibrary.PrintString` (`KismetSystemLibrary.GetDisplayName` _asfight_girl_bp))
      (`/Game/FSG/BLUEPRINTS/FightGIrlBP.PlayerTomarDaño` _asfight_girl_bp (`self.ReactionIndex`) (`self.HitboxDamage`)))))

(fn `UserConstructionScript`)