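; FSG game mode that runs the match timer and ends the game in a tie when time runs out.
; A Delay on Tick acts as a one-second clock, decrementing Countdown and rolling the Minutes and Seconds counters down.
; At zero it calls Lost, which sets GameOver and notifies the FSGGI game instance, then opens the TiePage level.
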(event `lost`
  (set `self.GameOver` true)
  (bind _asfsggi (cast `/Game/FSG/FSGGI` (`GameplayStatics.GetGameInstance`)))
  (`/Game/FSG/FSGGI.ENDGAMEINSTANCE` _asfsggi))

(event `self.ReceiveTick`
  (params (DeltaSeconds :type "Float (single-precision)"))
  ;[1 1 1] CONTADORES
  (`KismetSystemLibrary.Delay` 1.0)
  (set `self.Countdown` (- (`self.Countdown`) 1))
  (if (== (`self.Seconds`) 0)
    (if (== (`self.Minutes`) 0)
      (`self.lost`)
      (`GameplayStatics.OpenLevel` "TiePage")
      (else
        (set `self.Seconds` 59)
        (set `self.Minutes` (- (`self.Minutes`) 1))))
    (else
      (set `self.Seconds` (- (`self.Seconds`) 1)))))

(fn `UserConstructionScript`)