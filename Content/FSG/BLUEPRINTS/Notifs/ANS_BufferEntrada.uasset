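; Anim notify state that marks an input-buffer window on an animation, shown as "BuffEntrada" in the editor.
; On begin it finds the AC_BufferEntrada component on the mesh owner and calls AbrirBuffer to open the buffer.
; On end it calls CerrarBuffer on that same component to close it, doing nothing if the component is absent.
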(fn `GetNotifyName`
  (returns (ReturnValue :type String))
  (return "BuffEntrada"))

(fn `Received_NotifyBegin`
  (params (MeshComp :type "SkeletalMeshComponent Object Reference") (Animation :type "AnimSequenceBase Object Reference") (TotalDuration :type "Float (double-precision)"))
  (returns (ReturnValue :type Boolean))
  (bind _returnvalue (`Actor.GetComponentByClass` (`ActorComponent.GetOwner` MeshComp) "/Game/FSG/BLUEPRINTS/ACTORCOMP/AC_BufferEntrada.AC_BufferEntrada_C"))
  (`/Engine/EditorBlueprintResources/StandardMacros.IsValid` _returnvalue
    (:`Is Valid`
      (`/Game/FSG/BLUEPRINTS/ACTORCOMP/AC_BufferEntrada.AbrirBuffer` _returnvalue)
      (return false))))

(fn `Received_NotifyEnd`
  (params (MeshComp :type "SkeletalMeshComponent Object Reference") (Animation :type "AnimSequenceBase Object Reference"))
  (returns (ReturnValue :type Boolean))
  (bind _returnvalue (`Actor.GetComponentByClass` (`ActorComponent.GetOwner` MeshComp) "/Game/FSG/BLUEPRINTS/ACTORCOMP/AC_BufferEntrada.AC_BufferEntrada_C"))
  (`/Engine/EditorBlueprintResources/StandardMacros.IsValid` _returnvalue
    (:`Is Valid`
      (`/Game/FSG/BLUEPRINTS/ACTORCOMP/AC_BufferEntrada.CerrarBuffer` _returnvalue)
      (return false))))