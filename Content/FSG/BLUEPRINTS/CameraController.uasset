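; Camera actor that frames the player and an enemy, taking over player 0's view target on BeginPlay.
; Each Tick it centers itself on the Y and Z midpoint of PlayerRef and EnemigoRef.
; Its X position is a clamped remap of the distance between them, pulling farther into negative X as they separate, and the move is swept.
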(event `self.ReceiveBeginPlay`
  ;[1 0.84 0] Le quitamos el control de la camara al controlador del player y se lo otorgamos a este actor
  (`PlayerController.SetViewTargetWithBlend` (`GameplayStatics.GetPlayerController` 0) self 0.0 "VTBlend_Linear" 0.0 false))

(event `self.ReceiveTick`
  (params (DeltaSeconds :type "Float (single-precision)"))
  (bind (_returnvalue_x _returnvalue_y _returnvalue_z) (`KismetMathLibrary.BreakVector` (/ (+ (`self.K2_GetActorLocation` (`self.PlayerRef`)) (`self.K2_GetActorLocation` (`self.EnemigoRef`))) 2.0)))
  (`self.K2_SetActorLocation` (`KismetMathLibrary.MakeVector` (`KismetMathLibrary.MapRangeClamped` (`KismetMathLibrary.Vector_Distance` (`self.K2_GetActorLocation` (`self.PlayerRef`)) (`self.K2_GetActorLocation` (`self.EnemigoRef`))) 100.0 900.0 -300.0 -550.0) _returnvalue_y _returnvalue_z) true))

(fn `UserConstructionScript`)