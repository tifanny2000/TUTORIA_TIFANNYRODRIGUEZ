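; Actor component that buffers attack input and validates combo sequences against a list of named combos.
; While open with combos enabled, it matches each new key to the step after the last executed one; while closed, keys are consumed immediately.
; Confirmed attacks are flagged as executed and their montage broadcast through a dispatcher, advancing a hit counter if the Dummy is under attack.
; Reset clears flags and state, then closes the buffer.
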(fn `AbrirBuffer`
  (set `self.EstaAbierto` true)
  (`self.ON_BufferAbierto`))

(fn `ActualizarKey`
  (params (NuevoKey :type "/Game/FSG/BLUEPRINTS/Enumerations/Enum_BufferEntrada Enum" :default "NewEnumerator0") (Combo :type "/Game/FSG/BLUEPRINTS/Enumerations/Enum_Combos Enum" :default "NewEnumerator0"))
  ;[1 0.6923 0] Establezco que combo ejecutare
  (`self.SetCombo` Combo)
  (set `self.KeyAlmacenado` NuevoKey)
  (if (`self.EstaAbierto`)
    ;[1 0.711 0] Se habilitan los combos y se verifica si la combinacion de ataques es correcta
    (if (`self.HabilitarSistemaCombo`)
      (`self.CheckSecuenciaCombo` (`self.KeyAlmacenado`)))
    (else
      (`self.ConsumirBuffer`))))

(fn `CerrarBuffer`
  ;[1 0.7645 0] Solo se valida si se esta ejecutando un combo si se Habilita el uso del sistema
  (if (`self.HabilitarSistemaCombo`)
    (if (not (`self.EnCombo`))
      (set `self.EstaAbierto` false :!label _label)
      (`self.ON_BufferCerrado`))
    (else
      (goto _label))))

(fn `CheckSecuenciaCombo`
  (params (NewKey :type "/Game/FSG/BLUEPRINTS/Enumerations/Enum_BufferEntrada Enum" :default "NewEnumerator0"))
  (locals (L_LastIndex :type Integer) (L_NewIndex :type Integer) (L_SecAnterior :type Boolean))
  (set `local.L_SecAnterior` false)
  ;[1 0.7731 0] Se busca el item que contenga el combo que necesitamos, la busqueda se hace por nombre
  (for _array_element (`self.ListaCombos`)
    (bind (_nombre _secuencia) (break `/Game/FSG/BLUEPRINTS/Estructuras/F_Combos` _array_element))
    (if (`|EnumEquality` _nombre (`self.ComboActual`))
      ;[1 0.7969 0] Se busca que el ataque anterior se haya ejecutado y se guarda su index. La busqueda se hace por nombre del Input y tambien por ejecucion
      (for (_array_element_2 _array_index) _secuencia
        (bind (_inputkey _montage _ejecutado) (break `/Game/FSG/BLUEPRINTS/Estructuras/F_InfoCombo` _array_element_2))
        (if (and _ejecutado (`|EnumEquality` _inputkey (`self.AntKeyAlmacenado`)))
          (set `local.L_LastIndex` _array_index)
          (set `local.L_SecAnterior` true)
          (break)))
      ;[1 0.775 0] Si se ejecuto correctamente el ataque anterior entonces buscamos que el siguiente ataque sea igual al que queremos ejecutar en este momento. Ademas se confirma el ataque y se alamacena el ataque
      (if (`local.L_SecAnterior`)
        (if (`|EnumEquality` (`.InputKey_11_52F01142404A534B9B01EC9294A50F80` (break `/Game/FSG/BLUEPRINTS/Estructuras/F_InfoCombo` (`|GetArrayItem` _secuencia (+ (`local.L_LastIndex`) 1)))) (`local.NewKey`))
          (set `self.AntKeyAlmacenado` (`self.KeyAlmacenado`))
          (set `self.AtaqueConfirmado` true)
          (break)
          (else
            (set `self.ComboActual` "NewEnumerator0")
            (set `self.EnCombo` false)))
        (else
          (set `self.EnCombo` false)
          (break)))))
  (return))

(fn `ConfirmarAtaque`
  (if (`self.AtaqueConfirmado`)
    (set `self.AtaqueConfirmado` false)
    ;[1 0.802 0] Obtengo el montaje del combo y tambien actualizo si se ejecuto en la LISTACOMBOS. Y reproduzco el montage en el Player
    (set `self.EnCombo` true)
    (bind _montage (`self.GetMontage` (`self.ComboActual`) (`self.AntKeyAlmacenado`)))
    (`self.ON_PlayMontage` _montage)
    (bind _returnvalue (`GameplayStatics.GetActorOfClass` "/Game/FSG/BLUEPRINTS/AI/Dummy.Dummy_C"))
    (if (`/Game/FSG/BLUEPRINTS/AI/Dummy.BajoAtaque` _returnvalue)
      (set `self.ActivateCounter` true)
      ;[1 1 1] Counter de combo
      (set `self.Counter` (+ (`self.Counter`) 1))
      (set `self.CounterTotal` (+ (`self.CounterTotal`) 0)))))

(fn `ConsumirBuffer`
  (`self.ON_BufferConsumido` (`self.KeyAlmacenado`))
  (set `self.AntKeyAlmacenado` (`self.KeyAlmacenado`))
  (set `self.KeyAlmacenado` "NewEnumerator0"))

(fn `GetKeyAlmacenado`
  (returns (KeyAlmacenado :type "/Game/FSG/BLUEPRINTS/Enumerations/Enum_BufferEntrada Enum"))
  (return (`self.KeyAlmacenado`)))

(fn `GetMontage`
  (params (Combo :type "/Game/FSG/BLUEPRINTS/Enumerations/Enum_Combos Enum" :default "NewEnumerator0") (Key :type "/Game/FSG/BLUEPRINTS/Enumerations/Enum_BufferEntrada Enum" :default "NewEnumerator0"))
  (returns (Montage :type "AnimMontage Object Reference"))
  (locals (L_Montage :type "AnimMontage Object Reference") (L_ComboIndex :type Integer) (L_AttackIndex :type Integer))
  (set `local.L_Montage` null)
  (for (_array_element _array_index) (`self.ListaCombos`)
    (set `local.L_ComboIndex` _array_index)
    (bind (_nombre _secuencia) (break `/Game/FSG/BLUEPRINTS/Estructuras/F_Combos` _array_element))
    (if (`|EnumEquality` _nombre (`local.Combo`))
      (for (_array_element_2 _array_index_2) _secuencia
        (set `local.L_AttackIndex` _array_index_2)
        (bind ((`InputKey_11_52F01142404A534B9B01EC9294A50F80` _inputkey) (`Montage_10_64A01EC84AB293043B175E8302280422` _montage)) (break `/Game/FSG/BLUEPRINTS/Estructuras/F_InfoCombo` _array_element_2))
        (if (`|EnumEquality` _inputkey (`local.Key`))
          (setmembers `/Game/FSG/BLUEPRINTS/Estructuras/F_InfoCombo` :`StructRef` (`|GetArrayItem` (`.Secuencia_6_AB3F741A400346BFC644D8AFB8BA30A0` (break `/Game/FSG/BLUEPRINTS/Estructuras/F_Combos` (`|GetArrayItem` (`self.ListaCombos`) (`local.L_ComboIndex`)))) (`local.L_AttackIndex`)) :`Ejecutado` true)
          (set `local.L_Montage` _montage)
          (break)))
      (break)))
  (return (`local.L_Montage`)))

(fn `ResetCombo`
  (locals (L_ComboIndex :type Integer))
  ;[1 0.8667 0] Se reinicia la ejecucion a FALSE de todos los combos y ataques
  (for (_array_element _array_index) (`self.ListaCombos`)
    (set `local.L_ComboIndex` _array_index)
    (for (_ _array_index_2) (`.Secuencia_6_AB3F741A400346BFC644D8AFB8BA30A0` (break `/Game/FSG/BLUEPRINTS/Estructuras/F_Combos` _array_element))
      (setmembers `/Game/FSG/BLUEPRINTS/Estructuras/F_InfoCombo` :`StructRef` (`|GetArrayItem` (`.Secuencia_6_AB3F741A400346BFC644D8AFB8BA30A0` (break `/Game/FSG/BLUEPRINTS/Estructuras/F_Combos` (`|GetArrayItem` (`self.ListaCombos`) (`local.L_ComboIndex`)))) _array_index_2) :`Ejecutado` false)))
  ;[1 0.8735 0] Se reinician las variables y se cierra el bufer
  (set `self.AntKeyAlmacenado` "NewEnumerator0")
  (set `self.KeyAlmacenado` "NewEnumerator0")
  (set `self.AtaqueConfirmado` false)
  (set `self.ComboActual` "NewEnumerator0")
  (set `self.EnCombo` false)
  (set `self.ActivateCounter` false)
  (`self.CerrarBuffer`)
  (set `self.Counter` 1))

(fn `SetCombo`
  (params (NuevoCombo :type "/Game/FSG/BLUEPRINTS/Enumerations/Enum_Combos Enum" :default "NewEnumerator0"))
  ;[1 0.7709 0] Solo se actualizar el combo actual cuando el anterior es None
  (if (`|EnumEquality` (`self.ComboActual`) "NewEnumerator0")
    (set `self.ComboActual` NuevoCombo)
    ;[1 1 1] Se actualiza el primer ataque del combo seleccionado. El estado Ejecutado a TRUE
    (for (_array_element _array_index) (`self.ListaCombos`)
      (if (`|EnumEquality` (`.Nombre_2_B03C6D2C4F4080B049C7E0A5248E2ADF` (break `/Game/FSG/BLUEPRINTS/Estructuras/F_Combos` _array_element)) (`self.ComboActual`))
        (setmembers `/Game/FSG/BLUEPRINTS/Estructuras/F_InfoCombo` :`StructRef` (`|GetArrayItem` (`.Secuencia_6_AB3F741A400346BFC644D8AFB8BA30A0` (break `/Game/FSG/BLUEPRINTS/Estructuras/F_Combos` (`|GetArrayItem` (`self.ListaCombos`) _array_index)))) :`Ejecutado` true)
        (break)))))