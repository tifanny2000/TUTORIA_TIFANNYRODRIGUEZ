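; Actor component that buffers recent key presses and detects named command sequences, in the style of fighting-game inputs.
; RecibirInput prunes entries older than a short time window, then stores the key's display name and timestamp.
; CheckInputKeys scans the buffer for consecutive matches against each ListaComandos entry.
; A match calls IniciarComando, which flags the command used, sets ComboEjecutado and prints its name; ResetComando clears the per-command flags.
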(fn `AddlInputKeys`
  (params (InfoInput :type "/Game/FSG/BLUEPRINTS/Estructuras/F_InfoInput Structure (by ref)"))
  (`KismetArrayLibrary.Array_Add` (`self.InputKeys`) InfoInput)
  (`self.CheckInputKeys`))

(fn `AtaqueConfirmado`)

(fn `CheckInputKeys`
  (locals (L_ContadorSecuencia :type Integer))
  (bind _inputkeys (`self.InputKeys`))
  (for _array_element (`self.ListaComandos`)
    (bind (_nombre _inputs) (break `/Game/FSG/BLUEPRINTS/Estructuras/F_InfoComandos` _array_element))
    (for _array_element_2 _inputs
      (for (_ _array_index) _inputkeys
        (bind _returnvalue (+ _array_index (`local.L_ContadorSecuencia`)))
        (if (< _returnvalue (`KismetArrayLibrary.Array_Length` _inputkeys))
          (if (`KismetStringLibrary.EqualEqual_StrStr` (`.InputName_2_2ED839724BFBE7195EE8EDBE5729B96B` (break `/Game/FSG/BLUEPRINTS/Estructuras/F_InfoInput` (`|GetArrayItem` (`self.InputKeys`) _returnvalue))) _array_element_2)
            (bind _result (`/Engine/EditorBlueprintResources/StandardMacros.IncrementInt` (`local.L_ContadorSecuencia`))
              (:`  `
                (if (== _result (`KismetArrayLibrary.Array_Length` _inputs))
                  (`self.IniciarComando` _nombre)
                  (break)
                  (else
                    (break)))))
            (else
              (set `local.L_ContadorSecuencia` 0)))
          (else
            (set `local.L_ContadorSecuencia` 0)))))))

(fn `IniciarComando`
  (params (NombreComando :type String))
  (bind _listacomandos (`self.ListaComandos`))
  (for (_array_element _array_index) _listacomandos
    (bind _nombre (break `/Game/FSG/BLUEPRINTS/Estructuras/F_InfoComandos` _array_element))
    (if (`KismetStringLibrary.EqualEqual_StrStr` _nombre NombreComando)
      (setmembers `/Game/FSG/BLUEPRINTS/Estructuras/F_InfoComandos` :`StructRef` (`|GetArrayItem` _listacomandos _array_index) :`HaUsadoComando` true)
      (set `self.ComboEjecutado` true)
      (`KismetSystemLibrary.PrintString` _nombre true true (struct :`R` 1.0 :`G` 0.052534 :`A` 1.0)))))

(fn `NewFunction_0`)

(fn `RecibirInput`
  (params (Key :type "Key Structure" :default "None") (Tiempo :type "Float (double-precision)"))
  (bind _inputkeys (`self.InputKeys`))
  (for _array_element _inputkeys
    (if (< (`.TiempoEjecucion_6_30D0BAE04E6EC4A853505A8F1DDA6A23` (break `/Game/FSG/BLUEPRINTS/Estructuras/F_InfoInput` _array_element)) (- Tiempo 0.4))
      (`KismetArrayLibrary.Array_RemoveItem` _inputkeys _array_element)))
  (`self.AddlInputKeys` (make `/Game/FSG/BLUEPRINTS/Estructuras/F_InfoInput` (`KismetTextLibrary.Conv_TextToString` (`KismetInputLibrary.Key_GetDisplayName` Key)) (`local.Tiempo`))))

(fn `ResetComando`
  (bind _listacomandos (`self.ListaComandos`))
  (for _index (range (`KismetArrayLibrary.Array_Length` _listacomandos))
    (setmembers `/Game/FSG/BLUEPRINTS/Estructuras/F_InfoComandos` :`StructRef` (`|GetArrayItem` _listacomandos _index) :`HaUsadoComando` false)))