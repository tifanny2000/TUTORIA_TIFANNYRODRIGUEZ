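; Actor component that manages its owner's current state (Estado) as an enum, with functions to set, read and reset it.
; SetEstado cancels any SetIdle timer and stores the new state, but its state-changed notification is disconnected and never runs.
; ResetEstado skips one protected state, otherwise returns to idle immediately or starts a one-shot timer for the given delay.
; SetIdle applies the default enum value and prints a debug string.
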(fn `GetEstado`
  (returns (`Estado Actual` :type "/Game/FSG/BLUEPRINTS/Enumerations/Enum_BufferEstados Enum"))
  (return (`self.Estado Actual`)))

(fn `ResetEstado`
  (params (Tiempo :type "Float (double-precision)"))
  (if (`|EnumInequality` (`self.GetEstado`) "NewEnumerator5")
    (if (<= (`local.Tiempo`) 0.0)
      (`self.SetIdle`)
      (else
        (`KismetSystemLibrary.K2_SetTimerDelegate` (`|CreateDelegate` :!event `SetIdle`) (`local.Tiempo`))))))

(fn `SetEstado`
  (params (NuevoEstado :type "/Game/FSG/BLUEPRINTS/Enumerations/Enum_BufferEstados Enum" :default "NewEnumerator0"))
  (locals (L_EstadoPrev :type "/Game/FSG/BLUEPRINTS/Enumerations/Enum_BufferEstados Enum" :default "NewEnumerator0"))
  (`KismetSystemLibrary.K2_ClearTimer` null "SetIdle")
  (set `local.L_EstadoPrev` (`self.Estado Actual`))
  (bind _output_get (set `self.Estado Actual` NuevoEstado)))

(fn `SetIdle`
  (`self.SetEstado` "NewEnumerator0")
  (`KismetSystemLibrary.PrintString` "idle"))